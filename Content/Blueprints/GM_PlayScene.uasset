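; GM_PlayScene is the play scene's game mode Blueprint, providing the logic to spawn or respawn a player at a random Player Start.
; SpawnPlayer destroys the controller's current pawn if valid, then spawns a BP_PlayerCharacter and has the controller possess it.
; FindRandomPlayerStart supplies the spawn transform by picking randomly among all PlayerStart actors, with no check for occupancy.
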(fn `FindRandomPlayerStart`
  (returns (PlayerStartTransform :type "Transform Structure (by ref)"))
  (bind _outactors (`GameplayStatics.GetAllActorsOfClass` "/Script/Engine.PlayerStart"))
  (return (`self.GetTransform` (`KismetArrayLibrary.Array_Random` _outactors))))

(fn `SpawnPlayer`
  (params (PlayerController :type "PlayerController Object Reference"))
  (bind _returnvalue (`Controller.K2_GetPawn` PlayerController))
  (`/Engine/EditorBlueprintResources/StandardMacros.IsValid` _returnvalue
    (:`Is Valid`
      (`self.K2_DestroyActor` _returnvalue))
    (:`Is Not Valid`
      _))
  (bind _returnvalue_2 (`|SpawnActorFromClass` "/Game/Player/Blueprints/BP_PlayerCharacter.BP_PlayerCharacter_C" (`self.FindRandomPlayerStart`) "Undefined" "MultiplyWithRoot" null null))
  (`Controller.Possess` PlayerController _returnvalue_2))

(fn `UserConstructionScript`)